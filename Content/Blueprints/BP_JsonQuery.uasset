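; BP_JsonQuery is a helper Blueprint that loads and saves JSON files through a shared JsonData object.
; ReadJson creates a fresh JsonData and fills it from the configured read path, which is relative to the Content folder.
; WriteJson serializes JsonData to a string and saves it to the configured write path, with optional overwrite.
; Both store a success flag and print the path and result.
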(fn ConstructionScript)

(fn ReadJson
  (bind _readfile (Variables|Default|GetReadFile))
  (bind _readfilepath (Variables|Default|GetReadFilePath))
  (bind _returnvalue (Utilities|String|Append _readfilepath _readfile))
  (bind _output_get (Variables|Default|SetJsonData (Class|JsonFieldData|Create)))
  (bind _returnvalue_2 (Class|JsonFieldData|FromFile _output_get _returnvalue))
  (bind _output_get_2 (Variables|Default|SetIsRead _returnvalue_2))
  (Development|PrintString (Utilities|String|Append "Read " _returnvalue " : " (Utilities|String|ToString(Boolean) _output_get_2))))

(fn WriteJson
  (bind _writefile (Variables|Default|GetWriteFile))
  (bind _writefilepath (Variables|Default|GetWriteFilePath))
  (bind _returnvalue (Class|JsonFieldData|SaveStringTexttoFile _writefilepath _writefile (Class|JsonFieldData|ToString (Variables|Default|GetJsonData)) (Variables|Default|GetAllowOverwrite)))
  (bind _output_get (Variables|Default|SetIsWritten _returnvalue))
  (Development|PrintString (Utilities|String|Append "Write " (Utilities|String|Append _writefilepath _writefile) " : " (Utilities|String|ToString(Boolean) _output_get))))